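; A door that vanishes behind a wall once the first-person character passes into a trigger volume.
; Overlapping the OpenDoor volume enables input and opens a Gate, so pressing Interact plays a timeline that swings the door open on yaw.
; Entering WallBox shows the Wall, which starts without collision, makes it solid, and destroys the door and both trigger components.
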(event `self.ReceiveBeginPlay`
  (`PrimitiveComponent.SetCollisionEnabled` (`self.wall`) "NoCollision"))

(event `InputAction|Interact`
  (params (Key :type "Key Structure"))
  ;[1 1 1] Open Door
  (:`Pressed`
    (`/Engine/EditorBlueprintResources/StandardMacros.Gate` true :!label _label
      (:`Exit`
        (bind (_direction _doortrack) (`Timeline|Door_Timeline`)
          (:`Update`
            (`SceneComponent.K2_SetRelativeRotation` (`self.Door`) (`KismetMathLibrary.MakeRotator` 0.0 0.0 (`KismetMathLibrary.Lerp` 0.0 100.0 _doortrack)) false false)))))))

(event `self.OpenDoor.OnComponentBeginOverlap`
  (params (OverlappedComponent :type "PrimitiveComponent Object Reference") (OtherActor :type "Actor Object Reference") (OtherComp :type "PrimitiveComponent Object Reference") (OtherBodyIndex :type Integer) (bFromSweep :type Boolean) (SweepResult :type "HitResult Structure (by ref)"))
  ;[1 1 1] Open Door
  (cast `/Game/FirstPersonBP/Blueprints/FirstPersonCharacter` OtherActor)
  (`self.EnableInput` (`GameplayStatics.GetPlayerController` 0))
  (goto _label :!via `Open`))

(event `self.OpenDoor.OnComponentEndOverlap`
  (params (OverlappedComponent :type "PrimitiveComponent Object Reference") (OtherActor :type "Actor Object Reference") (OtherComp :type "PrimitiveComponent Object Reference") (OtherBodyIndex :type Integer))
  ;[1 1 1] Open Door
  (cast `/Game/FirstPersonBP/Blueprints/FirstPersonCharacter` OtherActor)
  (`self.DisableInput` (`GameplayStatics.GetPlayerController` 0))
  (goto _label :!via `Close`))

(event `self.WallBox.OnComponentBeginOverlap`
  (params (OverlappedComponent :type "PrimitiveComponent Object Reference") (OtherActor :type "Actor Object Reference") (OtherComp :type "PrimitiveComponent Object Reference") (OtherBodyIndex :type Integer) (bFromSweep :type Boolean) (SweepResult :type "HitResult Structure (by ref)"))
  (bind _wall (`self.wall`))
  (cast `/Game/FirstPersonBP/Blueprints/FirstPersonCharacter` OtherActor)
  (`SceneComponent.SetVisibility` _wall true false)
  (`PrimitiveComponent.SetCollisionEnabled` _wall "QueryAndPhysics")
  (`ActorComponent.K2_DestroyComponent` (`self.Door`))
  (`ActorComponent.K2_DestroyComponent` (`self.OpenDoor`))
  (`ActorComponent.K2_DestroyComponent` (`self.WallBox`)))

(fn `UserConstructionScript`)