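; Blockout box actor named as a correct tile for a jump tile puzzle; it builds its geometry procedurally and has no puzzle logic here.
; The construction script rounds BoxSize using RoundSize, adds the box, then calls BlockoutSetMaterial.
; AddBlockoutBox creates a static mesh component from BlockoutBoxMesh, scaling it by BoxSize divided by 100 to convert centimeter dimensions to mesh scale.
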(fn `AddBlockoutBox`
  (bind _returnvalue (`AddComponent|NODE_AddStaticMeshComponent-0` :`RelativeTransform` (`KismetMathLibrary.MakeTransform` (0.0 0.0 0.0) (struct) (* (`self.BoxSize`) (/ 1.0 100.0)))))
  (`StaticMeshComponent.SetStaticMesh` _returnvalue (`self.BlockoutBoxMesh`)))

(fn `UserConstructionScript`
  (`/BlockoutToolsPlugin/Blueprints/Utility/BlockoutToolsFunctions.BlockoutRoundVector` (`self.bRoundSize`) (`self.BoxSize`))
  (`self.AddBlockoutBox`)
  (`self.BlockoutSetMaterial`))