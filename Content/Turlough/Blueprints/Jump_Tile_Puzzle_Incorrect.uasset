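; Jump puzzle tile marked as incorrect, which destroys itself when the first-person character overlaps its Box component.
; The construction script rounds the box size, adds a static mesh component scaled from that size and applies the blockout material, so the tile is a resizable blockout box.
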(event `self.Box.OnComponentBeginOverlap`
  (params (OverlappedComponent :type "PrimitiveComponent Object Reference") (OtherActor :type "Actor Object Reference") (OtherComp :type "PrimitiveComponent Object Reference") (OtherBodyIndex :type Integer) (bFromSweep :type Boolean) (SweepResult :type "HitResult Structure (by ref)"))
  (cast `/Game/FirstPersonBP/Blueprints/FirstPersonCharacter` OtherActor)
  (`self.K2_DestroyActor`))

(fn `AddBlockoutBox`
  (bind _returnvalue (`AddComponent|NODE_AddStaticMeshComponent-0` :`RelativeTransform` (`KismetMathLibrary.MakeTransform` (0.0 0.0 0.0) (struct) (* (`self.BoxSize`) (/ 1.0 100.0)))))
  (`StaticMeshComponent.SetStaticMesh` _returnvalue (`self.BlockoutBoxMesh`)))

(fn `UserConstructionScript`
  (`/BlockoutToolsPlugin/Blueprints/Utility/BlockoutToolsFunctions.BlockoutRoundVector` (`self.bRoundSize`) (`self.BoxSize`))
  (`self.AddBlockoutBox`)
  (`self.BlockoutSetMaterial`))