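; MoveableObject is an actor with a cube that only simulates physics while the player is near it.
; A Box trigger switches physics on when a FirstPersonCharacter begins overlapping and off when it stops.
; On BeginPlay, two decals take their visibility from a shared flag and each receives its own configurable material.
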(event `self.ReceiveBeginPlay`
  (bind _decal (`self.Decal`))
  (`SceneComponent.SetVisibility` _decal (`self.DecalVisable?`) false)
  (`SceneComponent.SetVisibility` (`self.Decal`) (`self.DecalVisable?`) false)
  (`SceneComponent.SetVisibility` (`self.Decal1`) (`self.DecalVisable?`) false)
  (`DecalComponent.SetDecalMaterial` _decal (`self.Decal Material`))
  (`DecalComponent.SetDecalMaterial` (`self.Decal1`) (`self.Decal2 Material`)))

(event `self.Box.OnComponentBeginOverlap`
  (params (OverlappedComponent :type "PrimitiveComponent Object Reference") (OtherActor :type "Actor Object Reference") (OtherComp :type "PrimitiveComponent Object Reference") (OtherBodyIndex :type Integer) (bFromSweep :type Boolean) (SweepResult :type "HitResult Structure (by ref)"))
  (cast `/Game/FirstPersonBP/Blueprints/FirstPersonCharacter` OtherActor)
  (`PrimitiveComponent.SetSimulatePhysics` (`self.Cube`) true))

(event `self.Box.OnComponentEndOverlap`
  (params (OverlappedComponent :type "PrimitiveComponent Object Reference") (OtherActor :type "Actor Object Reference") (OtherComp :type "PrimitiveComponent Object Reference") (OtherBodyIndex :type Integer))
  (cast `/Game/FirstPersonBP/Blueprints/FirstPersonCharacter` OtherActor)
  (`PrimitiveComponent.SetSimulatePhysics` (`self.Cube`) false))

(fn `UserConstructionScript`)