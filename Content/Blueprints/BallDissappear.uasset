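; BallDissappear is a trigger actor that shows a set of actors while the first-person character is inside its Box and hides them on exit.
; Box begin and end overlap events filter for FirstPersonCharacter, then loop over MeshArray to set each root component's visibility.
; The visibility change does not propagate to child components, and nothing in the graph sets an initial hidden state.
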(event `self.Box.OnComponentBeginOverlap`
  (params (OverlappedComponent :type "PrimitiveComponent Object Reference") (OtherActor :type "Actor Object Reference") (OtherComp :type "PrimitiveComponent Object Reference") (OtherBodyIndex :type Integer) (bFromSweep :type Boolean) (SweepResult :type "HitResult Structure (by ref)"))
  (cast `/Game/FirstPersonBP/Blueprints/FirstPersonCharacter` OtherActor)
  (for _array_element (`self.Mesh Array`)
    (`SceneComponent.SetVisibility` (`Actor.RootComponent` _array_element) true false)))

(event `self.Box.OnComponentEndOverlap`
  (params (OverlappedComponent :type "PrimitiveComponent Object Reference") (OtherActor :type "Actor Object Reference") (OtherComp :type "PrimitiveComponent Object Reference") (OtherBodyIndex :type Integer))
  (cast `/Game/FirstPersonBP/Blueprints/FirstPersonCharacter` OtherActor)
  (for _array_element (`self.Mesh Array`)
    (`SceneComponent.SetVisibility` (`Actor.RootComponent` _array_element) false false)))

(fn `UserConstructionScript`)