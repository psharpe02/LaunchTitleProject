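; Ceiling light that flickers its spotlight after a random startup delay when its LightSwitch enum is set to the matching mode.
; BeginPlay passes a random time to the FlickeringLoop event, which feeds a collapsed flicker graph.
; A FasterLight flag picks one of two timelines to drive the SpotLight's IES brightness scale.
; Only the timeline used without FasterLight receives the random time.
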(event `self.ReceiveBeginPlay`
  (bind _returnvalue (`KismetMathLibrary.RandomFloatInRange` 2.0 10.0))
  (`|ExecutionSequence`
    (:`then_0`
      (`KismetSystemLibrary.Delay` _returnvalue)
      (`self.FlickeringLoop` _returnvalue))))

(event `FlickeringLoop`
  (params (NewTime :type "Float (double-precision)"))
  (if (`|EnumEquality` (`self.Light Switch`) "NewEnumerator2")
    (if (`self.Faster Light?`)
      (bind (_direction _value) (`Timeline|Timeline_1`)
        (:`Update`
          (`LightComponent.SetIESBrightnessScale` (`self.SpotLight`) _value)))
      (else
        (bind (_direction_2 _value_2) (`Timeline|Timeline_0` :`NewTime` NewTime)
          (:`Update`
            (`LightComponent.SetIESBrightnessScale` (`self.SpotLight`) _value_2)))))))

(fn `UserConstructionScript`)