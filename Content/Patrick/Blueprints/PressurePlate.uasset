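; Pressure plate puzzle switch that reports to its owning DoorMaster when weighted by a LetterCube or, in MazeDoorSwitch mode, a toy.
; Overlap sets the door's Locked flag and plays a plate timeline that updates material and Connectors, then adjusts the DoorSwitches array.
; LetterCube end overlap clears the flag and reverses the timeline.
; MazeDoorSwitch swaps meshes, shows proximity text and lets ItemPlace spawn-in the player's collected toy as a physics mesh.
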(event `self.ReceiveBeginPlay`
  (if (`self.MazeDoorSwitch?`)
    (`StaticMeshComponent.SetStaticMesh` (`self.PressurePlate`) "/Game/Patrick/Meshes/BlockoutAssets/PressurePlatetoy.PressurePlatetoy")
    (`StaticMeshComponent.SetStaticMesh` (`self.PressurePlate2`) "/Game/Patrick/Meshes/BlockoutAssets/PressurePlatetoy2.PressurePlatetoy2")
    (`SceneComponent.K2_SetRelativeLocation` (`self.PressurePlate2`) (`self.New Location`) false false)
    (`SceneComponent.K2_SetRelativeLocation` (`self.Box`) (`self.New Location_0`) false false)))

(event `self.ReceiveTick`
  (params (DeltaSeconds :type "Float (single-precision)"))
  (`|ExecutionSequence`
    (:`then_0`
      (bind _asfirst_person_character (cast `/Game/FirstPersonBP/Blueprints/FirstPersonCharacter` (`GameplayStatics.GetPlayerCharacter` 0)))
      (set `self.FPC` _asfirst_person_character))
    (:`then_1`
      (bind _asdoor_master (cast `/Game/Patrick/Blueprints/Interactable/DoorMaster` (`self.GetOwner`)))
      (set `self.As Door Master` _asdoor_master))))

(event `self.Box.OnComponentBeginOverlap`
  (params (OverlappedComponent :type "PrimitiveComponent Object Reference") (OtherActor :type "Actor Object Reference") (OtherComp :type "PrimitiveComponent Object Reference") (OtherBodyIndex :type Integer) (bFromSweep :type Boolean) (SweepResult :type "HitResult Structure (by ref)"))
  (bind _pressureplate2 (`self.PressurePlate2`))
  (bind _pressureplate2_2 (`self.PressurePlate2`))
  (bind _pressureplate2_3 (`self.PressurePlate2`))
  (bind _as_door_master (`self.As Door Master`))
  (bind _doornum (`/Game/Patrick/Blueprints/Interactable/DoorMaster.DoorNum` _as_door_master))
  (bind (_relativelocation_x _relativelocation_y) (`KismetMathLibrary.BreakVector` (`SceneComponent.RelativeLocation` _pressureplate2)))
  (bind _doorswitches_ (`/Game/Patrick/Blueprints/Interactable/DoorMaster.DoorSwitches?` _as_door_master))
  (bind (_relativelocation_x_2 _relativelocation_y_2) (`KismetMathLibrary.BreakVector` (`SceneComponent.RelativeLocation` _pressureplate2_3)))
  (bind _returnvalue (== (`KismetArrayLibrary.Array_LastIndex` _doorswitches_) _doornum))
  (if (`self.MazeDoorSwitch?`)
    (if (`PrimitiveComponent.IsOverlappingComponent` (`self.Box`) (`self.toymesh`))
      (set `/Game/Patrick/Blueprints/Interactable/DoorMaster.Locked?` true (`self.As Door Master`) :!label _label)
      (if (`self.MazeDoorSwitch?`)
        ;[1 1 1] Cube Door Pressure Plate
        (bind (_direction _value) (`Timeline|Timeline_1` :!label _label_2)
          (:`Update`
            (`SceneComponent.K2_SetRelativeLocation` _pressureplate2 (`KismetMathLibrary.MakeVector` _relativelocation_x _relativelocation_y _value) false false)
            (`KismetSystemLibrary.Delay` 1.0 :!label _label_3)
            (if (`/Game/Patrick/Blueprints/Interactable/DoorMaster.Locked?` (`self.As Door Master`))
              (`PrimitiveComponent.SetMaterial` _pressureplate2_2 0 "/Game/Materials/Dayna_Textures/plain_wall_MAT.plain_wall_MAT")
              (set `self.Connectors` 1)
              (set `self.Item Num` (+ (`self.Item Num`) 1))
              (else
                (`PrimitiveComponent.SetMaterial` _pressureplate2_2 0 "/Game/Materials/Dayna_Textures/Soft_puzzle_red_mat_MAT.Soft_puzzle_red_mat_MAT")
                (set `self.Connectors` 0))))
          (:`Finished`
            (if (`/Game/Patrick/Blueprints/Interactable/DoorMaster.Locked?` (`self.As Door Master`)) :!label _label_4
              (if (not _returnvalue)
                (`KismetArrayLibrary.Array_Add` _doorswitches_ true)
                (`KismetSystemLibrary.PrintString` "add"))
              (elif _returnvalue
                (`KismetArrayLibrary.Array_Remove` _doorswitches_ _doornum)
                (`KismetSystemLibrary.PrintString` "remove")
                (else
                  (`KismetSystemLibrary.PrintString` "clear"))))))
        (else
          (bind (_direction_2 _value_2) (`Timeline|Timeline_0` :!label _label_5)
            (:`Update`
              (`SceneComponent.K2_SetRelativeLocation` _pressureplate2_3 (`KismetMathLibrary.MakeVector` _relativelocation_x_2 _relativelocation_y_2 _value_2) false false)
              (goto _label_3))
            (:`Finished`
              (goto _label_4))))))
    (else
      (cast `/Game/Patrick/Blueprints/LetterCube` OtherActor)
      (goto _label))))

(event `self.Box.OnComponentEndOverlap`
  (params (OverlappedComponent :type "PrimitiveComponent Object Reference") (OtherActor :type "Actor Object Reference") (OtherComp :type "PrimitiveComponent Object Reference") (OtherBodyIndex :type Integer))
  (cast `/Game/Patrick/Blueprints/LetterCube` OtherActor)
  (set `/Game/Patrick/Blueprints/Interactable/DoorMaster.Locked?` false (`self.As Door Master`))
  (if (`self.MazeDoorSwitch?`)
    (goto _label_2 :!via `Reverse`)
    (else
      (goto _label_5 :!via `Reverse`))))

(event `ItemPlace`
  (bind _toymesh (`self.toymesh`))
  (bind _item_num (`self.Item Num`))
  ;[1 1 1] Item Placed
  (if (`self.MazeDoorSwitch?`)
    (bind _asfirst_person_character (cast `/Game/FirstPersonBP/Blueprints/FirstPersonCharacter` (`GameplayStatics.GetPlayerCharacter` 0)))
    (bind _itemcollect (`/Game/FirstPersonBP/Blueprints/FirstPersonCharacter.ItemCollect` _asfirst_person_character))
    (if (`KismetArrayLibrary.Array_IsValidIndex` _itemcollect _item_num)
      (if (== (`|GetArrayItem` _itemcollect _item_num) true)
        (`TextRenderComponent.K2_SetText` (`self.TextRender`) (`|GetArrayItem` (`self.Text`) 3))
        (`StaticMeshComponent.SetStaticMesh` (`self.toymesh`) (`self.Toy Item`))
        (`SceneComponent.SetVisibility` _toymesh true false)
        (`PrimitiveComponent.SetSimulatePhysics` _toymesh true))
      (else
        (`TextRenderComponent.K2_SetText` (`self.TextRender`) (`|GetArrayItem` (`self.Text`) 1))))))

(event `self.Box1.OnComponentBeginOverlap`
  (params (OverlappedComponent :type "PrimitiveComponent Object Reference") (OtherActor :type "Actor Object Reference") (OtherComp :type "PrimitiveComponent Object Reference") (OtherBodyIndex :type Integer) (bFromSweep :type Boolean) (SweepResult :type "HitResult Structure (by ref)"))
  ;[1 1 1] TextRenderCollision
  (if (`self.MazeDoorSwitch?`)
    (cast `/Game/FirstPersonBP/Blueprints/FirstPersonCharacter` OtherActor)
    (`SceneComponent.SetVisibility` (`self.TextRender`) true false)))

(event `self.Box1.OnComponentEndOverlap`
  (params (OverlappedComponent :type "PrimitiveComponent Object Reference") (OtherActor :type "Actor Object Reference") (OtherComp :type "PrimitiveComponent Object Reference") (OtherBodyIndex :type Integer))
  ;[1 1 1] TextRenderCollision
  (if (`self.MazeDoorSwitch?`)
    (cast `/Game/FirstPersonBP/Blueprints/FirstPersonCharacter` OtherActor)
    (`SceneComponent.SetVisibility` (`self.TextRender`) false false)
    (`TextRenderComponent.K2_SetText` (`self.TextRender`) (`|GetArrayItem` (`self.Text`)))))

(fn `UserConstructionScript`
  (if (`self.MazeDoorSwitch?`)
    (`StaticMeshComponent.SetStaticMesh` (`self.PressurePlate`) "/Game/Patrick/Meshes/BlockoutAssets/PressurePlatetoy.PressurePlatetoy")
    (`StaticMeshComponent.SetStaticMesh` (`self.PressurePlate2`) "/Game/Patrick/Meshes/BlockoutAssets/PressurePlatetoy2.PressurePlatetoy2")
    (`SceneComponent.K2_SetRelativeLocation` (`self.PressurePlate2`) (`self.New Location`) false false)
    (`SceneComponent.K2_SetRelativeLocation` (`self.Box`) (`self.New Location_0`) false false)
    (`SceneComponent.K2_SetRelativeLocation` (`self.Box1`) (`self.New Location_0`) false false)
    (else
      (`ActorComponent.K2_DestroyComponent` (`self.toymesh`))
      (`ActorComponent.K2_DestroyComponent` (`self.Box1`)))))