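; Interactable single or double door master Blueprint with per-instance meshes, jammed and banging states, and gating by switch or player key.
; The DoorMaster event checks those conditions and Locked, which reads inverted (true permits use), then toggles the swing timeline with sound.
; Leaving the trigger box reverses the swing after an interaction, closing the door.
; Tick updates the last light indicator's colour and plays the banging timeline.
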(event `self.ReceiveTick`
  (params (DeltaSeconds :type "Float (single-precision)"))
  (bind _light_indicator (`self.Light Indicator`))
  (bind _returnvalue (`KismetArrayLibrary.Array_LastIndex` _light_indicator))
  (bind _output (`|GetArrayItem` _light_indicator _returnvalue))
  ;[1 1 1] Event Tick
  (`|ExecutionSequence`
    (:`then_0`
      (bind _asfirst_person_character (cast `/Game/FirstPersonBP/Blueprints/FirstPersonCharacter` (`GameplayStatics.GetPlayerCharacter` 0)))
      (set `self.FPC` _asfirst_person_character)
      (if (`KismetArrayLibrary.Array_IsValidIndex` _light_indicator _returnvalue)
        (if (== (`KismetArrayLibrary.Array_LastIndex` (`self.DoorSwitches?`)) (`self.DoorNum`))
          (if (`self.Locked?`) :!label _label
            (set `/Game/Patrick/Blueprints/CircularLights.LightColours` "NewEnumerator0" _output)
            (else
              (set `/Game/Patrick/Blueprints/CircularLights.LightColours` "NewEnumerator1" _output :!label _label_2)))
          (elif (== (`KismetArrayLibrary.Array_LastIndex` (`/Game/FirstPersonBP/Blueprints/BaseCharacter_BP.Key?` (`self.FPC`))) (`self.DoorNum`))
            (goto _label)
            (else
              (goto _label_2))))))
    (:`then_1`
      (if (`self.Door Banging`)
        (bind (_direction _doorr _doorl) (`Timeline|Timeline_0`)
          (:`Update`
            (bind _output_get (set `self.DoorLOpenRotation` _doorl))
            (`SceneComponent.K2_SetRelativeRotation` (`self.DoorL`) (`KismetMathLibrary.MakeRotator` 0.0 0.0 (.z _output_get)) false false)
            (bind _output_get_2 (set `self.DoorROpenRotation` _doorr))
            (`SceneComponent.K2_SetRelativeRotation` (`self.DoorR`) (`KismetMathLibrary.MakeRotator` 0.0 0.0 (.z _output_get_2)) false false))
          (:`Finished`
            (`KismetSystemLibrary.Delay` (`self.Door Duration`))))))))

(event `DoorMaster`
  (bind _returnvalue (`self.K2_GetActorLocation`))
  (bind _doornum (`self.DoorNum`))
  (bind _doorswitches_ (`self.DoorSwitches?`))
  (bind _doornum_2 (`self.DoorNum`))
  (bind _key_ (`/Game/FirstPersonBP/Blueprints/BaseCharacter_BP.Key?` (`self.FPC`)))
  ;[1 1 1] Doors
  (set `self.DoorInteracted?` true)
  (if (`self.Jammed?`)
    (`KismetSystemLibrary.PrintString` "Door is jammed Can not enter!" true true (struct :`G` 0.66 :`B` 1.0 :`A` 1.0) 5.0)
    (elif (`KismetArrayLibrary.Array_IsValidIndex` _doorswitches_ _doornum_2)
      (if (`|GetArrayItem` _doorswitches_ _doornum_2)
        (if (`self.Door Banging`) :!label _label_3
          _
          (elif (`self.Locked?`)
            (if (`self.DoorOpen?`)
              (set `self.DoorOpen?` false)
              (`GameplayStatics.PlaySoundAtLocation` "/Game/sounds/Nicole/Sounds/DoorSounds.DoorSounds" _returnvalue (struct) 1.0 1.0 0.0 null null null)
              (bind (_direction _doorl _doorr) (`Timeline|Door Transition` :!label _label_4)
                (:`Update`
                  (bind _output_get (set `self.DoorLOpenRotation` _doorl))
                  (`SceneComponent.K2_SetRelativeRotation` (`self.DoorL`) (`KismetMathLibrary.MakeRotator` 0.0 0.0 (.z _output_get)) false false)
                  (bind _output_get_2 (set `self.DoorROpenRotation` _doorr))
                  (`SceneComponent.K2_SetRelativeRotation` (`self.DoorR`) (`KismetMathLibrary.MakeRotator` 0.0 0.0 (.z _output_get_2)) false false))
                (:`Finished`
                  (`KismetSystemLibrary.Delay` (`self.Door Duration`))))
              (else
                (set `self.DoorOpen?` true)
                (`GameplayStatics.PlaySoundAtLocation` "/Game/sounds/Nicole/Sounds/DoorSounds.DoorSounds" _returnvalue (struct) 1.0 1.0 0.0 null null null)
                (goto _label_4 :!via `Reverse`))))))
      (elif (`self.RequiresKey?`)
        (if (`KismetArrayLibrary.Array_IsValidIndex` _key_ _doornum)
          (if (`|GetArrayItem` _key_ _doornum)
            (goto _label_3)))))))

(event `self.Box1.OnComponentBeginOverlap`
  (params (OverlappedComponent :type "PrimitiveComponent Object Reference") (OtherActor :type "Actor Object Reference") (OtherComp :type "PrimitiveComponent Object Reference") (OtherBodyIndex :type Integer) (bFromSweep :type Boolean) (SweepResult :type "HitResult Structure (by ref)"))
  ;[1 1 1] Box Door Overlap
  (cast `/Game/FirstPersonBP/Blueprints/FirstPersonCharacter` OtherActor)
  (if (not (`self.Locked?`))
    (`KismetSystemLibrary.PrintString` "Door isn't unlocked yet")))

(event `self.Box1.OnComponentEndOverlap`
  (params (OverlappedComponent :type "PrimitiveComponent Object Reference") (OtherActor :type "Actor Object Reference") (OtherComp :type "PrimitiveComponent Object Reference") (OtherBodyIndex :type Integer))
  ;[1 1 1] Box Door Overlap
  (cast `/Game/FirstPersonBP/Blueprints/FirstPersonCharacter` OtherActor)
  (if (not (`self.DoorOpen?`))
    (set `self.DoorOpen?` true)
    (if (`self.DoorInteracted?`)
      (`GameplayStatics.PlaySoundAtLocation` "/Game/sounds/Nicole/Sounds/DoorSounds.DoorSounds" (`self.K2_GetActorLocation`) (struct) 1.0 1.0 0.0 null null null)
      (`TimelineComponent.Reverse` (`self.Door Transition`))
      (set `self.DoorInteracted?` false))))

(fn `UserConstructionScript`
  (bind _box1 (`self.Box1`))
  (`StaticMeshComponent.SetStaticMesh` (`self.DoorL`) (`self.Door MeshL`))
  (`StaticMeshComponent.SetStaticMesh` (`self.DoorR`) (`self.Door MeshR`))
  (if (`self.DoubleDoor?`)
    (`SceneComponent.SetVisibility` (`self.DoorR`) true false)
    (`SceneComponent.SetRelativeScale3D` _box1 (`self.Box Scale`))
    (`SceneComponent.K2_SetRelativeLocation` _box1 (`self.Box Location`) false false)))