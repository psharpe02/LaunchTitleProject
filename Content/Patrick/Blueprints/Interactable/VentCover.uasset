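; VentCover is an interactable that tells the first-person character when it can vent while holding a particular item.
; Overlapping its Box with item index 2 selected sets the character's Venting flag, and leaving with it selected clears the flag.
; Each side passes through its own DoOnce, which resets only when that overlap event occurs with another item selected.
; A Box DestroyComponent call is left unconnected.
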(event `self.Box.OnComponentBeginOverlap`
  (params (OverlappedComponent :type "PrimitiveComponent Object Reference") (OtherActor :type "Actor Object Reference") (OtherComp :type "PrimitiveComponent Object Reference") (OtherBodyIndex :type Integer) (bFromSweep :type Boolean) (SweepResult :type "HitResult Structure (by ref)"))
  (bind _asfirst_person_character (cast `/Game/FirstPersonBP/Blueprints/FirstPersonCharacter` OtherActor))
  (if (== (`/Game/FirstPersonBP/Blueprints/BaseCharacter_BP.SelectedItem` _asfirst_person_character) 2)
    (`/Engine/EditorBlueprintResources/StandardMacros.DoOnce` false :!label _label
      (:`Completed`
        (set `/Game/FirstPersonBP/Blueprints/BaseCharacter_BP.Venting?` true _asfirst_person_character)))
    (else
      (goto _label :!via `Reset`))))

(event `self.Box.OnComponentEndOverlap`
  (params (OverlappedComponent :type "PrimitiveComponent Object Reference") (OtherActor :type "Actor Object Reference") (OtherComp :type "PrimitiveComponent Object Reference") (OtherBodyIndex :type Integer))
  (bind _asfirst_person_character (cast `/Game/FirstPersonBP/Blueprints/FirstPersonCharacter` OtherActor))
  (if (== (`/Game/FirstPersonBP/Blueprints/BaseCharacter_BP.SelectedItem` _asfirst_person_character) 2)
    (`/Engine/EditorBlueprintResources/StandardMacros.DoOnce` false :!label _label_2
      (:`Completed`
        (set `/Game/FirstPersonBP/Blueprints/BaseCharacter_BP.Venting?` false _asfirst_person_character)))
    (else
      (goto _label_2 :!via `Reset`))))

(fn `UserConstructionScript`)