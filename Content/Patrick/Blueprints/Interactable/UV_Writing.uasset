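; UV_Writing is an interactable writing actor whose UVWriting text can be revealed and hidden, apparently as a UV-revealed message.
; The construction script fills the text component from the Text variable, so each instance can carry its own message.
; UVWritingActivate and UVWritingDeactivate toggle the component's visibility, each acting only when the state needs to change.
; BeginPlay caches the player's FirstPersonCharacter, though these graphs never use it.
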(event `self.ReceiveBeginPlay`
  (bind _asfirst_person_character (cast `/Game/FirstPersonBP/Blueprints/FirstPersonCharacter` (`GameplayStatics.GetPlayerCharacter` 0)))
  (set `self.FPC` _asfirst_person_character))

(event `UVWritingActivate`
  (bind _uv_writing (`self.UV Writing`))
  (if (not (`SceneComponent.bVisible` _uv_writing))
    (`SceneComponent.SetVisibility` _uv_writing true false)))

(event `UVWritingDeactivate`
  (if (`SceneComponent.bVisible` (`self.UV Writing`))
    (`SceneComponent.SetVisibility` (`self.UV Writing`) false false)))

(fn `UserConstructionScript`
  (`TextRenderComponent.K2_SetText` (`self.UV Writing`) (`self.Text`)))