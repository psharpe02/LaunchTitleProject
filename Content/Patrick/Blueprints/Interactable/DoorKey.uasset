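; DoorKey is an interactable door Blueprint that swings its RDoor component open and shut.
; BeginPlay applies a material to the door.
; Each DoorKey event flips the DoorOpen flag, playing a timeline when it was true and reversing it when false.
; The timeline's Rotation track lerps the door's relative yaw between 0 and -80 degrees during forward and reverse playback.
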(event `self.ReceiveBeginPlay`
  (`PrimitiveComponent.SetMaterial` (`self.RDoor`) 0 (`self.Material`)))

(event `DoorKey`
  (if (`self.DoorOpen?`)
    (set `self.DoorOpen?` false)
    (bind (_direction _rotation) (`Timeline|Timeline_0` :!label _label)
      (:`Update`
        (`SceneComponent.K2_SetRelativeRotation` (`self.RDoor`) (`KismetMathLibrary.MakeRotator` 0.0 0.0 (`KismetMathLibrary.Lerp` 0.0 -80.0 _rotation)) false false)))
    (else
      (set `self.DoorOpen?` true)
      (goto _label :!via `Reverse`))))

(fn `UserConstructionScript`)