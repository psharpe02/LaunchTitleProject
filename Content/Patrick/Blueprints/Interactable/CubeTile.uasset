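; CubeTile is an interactable tile that is solid and visible only while the first-person character's Tile flag is true.
; A Box overlap caches the FirstPersonCharacter and applies the state immediately; no end-overlap clears that reference.
; Tick re-reads the flag from the cached character every frame, switching the static mesh's collision and hidden-in-game state together.
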(event `self.ReceiveTick`
  (params (DeltaSeconds :type "Float (single-precision)"))
  (bind _staticmesh (`self.StaticMesh`))
  (if (`/Game/FirstPersonBP/Blueprints/BaseCharacter_BP.Tile?` (stale `self.Box.OnComponentBeginOverlap` _asfirst_person_character)) :!label _label
    (`PrimitiveComponent.SetCollisionEnabled` _staticmesh "QueryAndPhysics")
    (`SceneComponent.SetHiddenInGame` (`self.StaticMesh`) false false)
    (else
      (`PrimitiveComponent.SetCollisionEnabled` _staticmesh "NoCollision")
      (`SceneComponent.SetHiddenInGame` (`self.StaticMesh`) true false))))

(event `self.Box.OnComponentBeginOverlap`
  (params (OverlappedComponent :type "PrimitiveComponent Object Reference") (OtherActor :type "Actor Object Reference") (OtherComp :type "PrimitiveComponent Object Reference") (OtherBodyIndex :type Integer) (bFromSweep :type Boolean) (SweepResult :type "HitResult Structure (by ref)"))
  (bind _asfirst_person_character (cast `/Game/FirstPersonBP/Blueprints/FirstPersonCharacter` OtherActor))
  (goto _label))

(fn `UserConstructionScript`)