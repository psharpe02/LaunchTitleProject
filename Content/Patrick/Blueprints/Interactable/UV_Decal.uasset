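; UV_Decal is a decal actor for hidden UV writing that can be revealed and hidden during play.
; The construction script applies the configurable decal material, and BeginPlay caches the first-person character, then hides the decal.
; UVWritingActivate and UVWritingDeactivate events toggle its visibility, changing it only when the state differs; their callers live outside this Blueprint.
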(event `self.ReceiveBeginPlay`
  (bind _asfirst_person_character (cast `/Game/FirstPersonBP/Blueprints/FirstPersonCharacter` (`GameplayStatics.GetPlayerCharacter` 0)))
  (set `self.FPC` _asfirst_person_character)
  (`SceneComponent.SetVisibility` (`self.Decal`) false false))

(event `UVWritingActivate`
  (bind _decal (`self.Decal`))
  (if (not (`SceneComponent.bVisible` _decal))
    (`SceneComponent.SetVisibility` _decal true false)))

(event `UVWritingDeactivate`
  (bind _decal (`self.Decal`))
  (if (`SceneComponent.bVisible` _decal)
    (`SceneComponent.SetVisibility` _decal false false)))

(fn `UserConstructionScript`
  (`DecalComponent.SetDecalMaterial` (`self.Decal`) (`self.New Decal Material`)))