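; Interactable left double-door Blueprint that swings its LDoor component open and shut.
; BeginPlay applies the Material variable to the door mesh.
; Each DoorIteraction event flips DoorOpen and plays or reverses the OpenDoor timeline, whose Rotation track lerps the door's relative yaw between closed and 80 degrees.
; The flag reads inverted: DoorOpen being true triggers the forward swing and then becomes false.
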(event `self.ReceiveBeginPlay`
  (`PrimitiveComponent.SetMaterial` (`self.LDoor`) 0 (`self.Material`)))

(event `Door Iteraction`
  (if (`self.DoorOpen?`)
    (set `self.DoorOpen?` false)
    (bind (_direction _rotation) (`Timeline|OpenDoor` :!label _label)
      (:`Update`
        (`SceneComponent.K2_SetRelativeRotation` (`self.LDoor`) (`KismetMathLibrary.MakeRotator` 0.0 0.0 (`KismetMathLibrary.Lerp` 0.0 80.0 _rotation)) false false)))
    (else
      (set `self.DoorOpen?` true)
      (goto _label :!via `Reverse`))))

(fn `UserConstructionScript`)