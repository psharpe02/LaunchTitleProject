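; Elevator actor with configurable left and optional right door meshes, gated by jammed, switch and Locked states.
; The Elevator event toggles a scale timeline that slides the doors, which Tick also drives from Box1 overlap, alongside a banging rotation animation.
; Tick also sets a LightSwap colour from switch index.
; Box1 overlap flags the player's elevator state and, when Locked is true, triggers ElevatorLift up or down.
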(event `self.ReceiveBeginPlay`
  ;[1 1 1] Event Begin Play
  (`StaticMeshComponent.SetStaticMesh` (`self.DoorL`) (`self.DoorLMesh`))
  (`StaticMeshComponent.SetStaticMesh` (`self.DoorR`) (`self.DoorRMesh`)))

(event `self.ReceiveTick`
  (params (DeltaSeconds :type "Float (single-precision)"))
  (bind _door_transition (`self.Door Transition`))
  (bind _door_duration (`self.Door Duration`))
  (bind _light_swap (`self.Light Swap`))
  (bind _returnvalue (`KismetArrayLibrary.Array_Length` _light_swap))
  (bind _output (`|GetArrayItem` _light_swap _returnvalue))
  ;[1 1 1] Event Tick
  (`|ExecutionSequence`
    (:`then_0`
      (bind _asfirst_person_character (cast `/Game/FirstPersonBP/Blueprints/FirstPersonCharacter` (`GameplayStatics.GetPlayerCharacter` 0)))
      (set `self.FPC` _asfirst_person_character)
      (if (`KismetArrayLibrary.Array_IsValidIndex` _light_swap _returnvalue)
        (if (== (`KismetArrayLibrary.Array_LastIndex` (`self.DoorSwitches?`)) (`self.DoorNum`))
          (set `/Game/Patrick/Blueprints/CircularLights.LightColours` "NewEnumerator0" _output)
          (else
            (set `/Game/Patrick/Blueprints/CircularLights.LightColours` "NewEnumerator1" _output)))))
    (:`then_1`
      (if (`self.Door Banging`)
        (bind (_direction _doorl _doorr) (`Timeline|DoorBang`)
          (:`Update`
            (`SceneComponent.K2_SetRelativeRotation` (`self.DoorL`) (`KismetMathLibrary.MakeRotator` 0.0 0.0 (`KismetMathLibrary.Lerp` 0.0 10.0 _doorl)) false false)
            (`SceneComponent.K2_SetRelativeRotation` (`self.DoorR`) (`KismetMathLibrary.MakeRotator` 0.0 0.0 (`KismetMathLibrary.Lerp` 0.0 -15.0 _doorr)) false false)))))
    (:`then_2`
      (if (`PrimitiveComponent.IsOverlappingActor` (`self.Box1`) (`self.FPC`))
        (`KismetSystemLibrary.Delay` _door_duration)
        (`TimelineComponent.Play` _door_transition)
        (else
          (`KismetSystemLibrary.Delay` _door_duration)
          (`TimelineComponent.Reverse` _door_transition))))))

(event `Elevator`
  (bind _doorswitches_ (`self.DoorSwitches?`))
  (bind _doornum (`self.DoorNum`))
  ;[1 1 1] Locked DoorL
  (if (`self.Jammed?`)
    (`KismetSystemLibrary.PrintString` "There is something stuff under this elevator" true true (struct :`G` 0.66 :`B` 1.0 :`A` 1.0) 5.0)
    (elif (`KismetArrayLibrary.Array_IsValidIndex` _doorswitches_ _doornum)
      (if (`|GetArrayItem` _doorswitches_ _doornum)
        (if (`self.Door Banging`)
          _
          (elif (`self.Locked?`)
            (if (`self.DoorOpen?`)
              (set `self.DoorOpen?` false)
              (bind (_direction _doorl _doorr) (`Timeline|Door Transition` :!label _label)
                (:`Update`
                  (`SceneComponent.SetRelativeScale3D` (`self.DoorL`) (`KismetMathLibrary.MakeVector` (.x _doorl) 1.0 1.0))
                  (`SceneComponent.SetRelativeScale3D` (`self.DoorR`) (`KismetMathLibrary.MakeVector` (.x _doorr) 1.0 1.0))))
              (else
                (set `self.DoorOpen?` true)
                (goto _label :!via `Reverse`)))))))))

(event `self.Box1.OnComponentBeginOverlap`
  (params (OverlappedComponent :type "PrimitiveComponent Object Reference") (OtherActor :type "Actor Object Reference") (OtherComp :type "PrimitiveComponent Object Reference") (OtherBodyIndex :type Integer) (bFromSweep :type Boolean) (SweepResult :type "HitResult Structure (by ref)"))
  (bind _elevatorlift (`self.ElevatorLift`))
  (bind _asfirst_person_character (cast `/Game/FirstPersonBP/Blueprints/FirstPersonCharacter` OtherActor))
  (if (`self.Locked?`)
    (set `/Game/FirstPersonBP/Blueprints/FirstPersonCharacter.InElevator?` true _asfirst_person_character)
    (bind _output_get (set `/Game/FirstPersonBP/Blueprints/FirstPersonCharacter.ElevatorUp?` (`self.Elevator Up?`) _asfirst_person_character))
    (if _output_get
      (`/Game/Patrick/Blueprints/Interactable/ElevatorLift.Elevator Up` _elevatorlift)
      (else
        (`/Game/Patrick/Blueprints/Interactable/ElevatorLift.ElevatorDown` _elevatorlift)))
    (else
      (`KismetSystemLibrary.PrintString` "Door isn't unlocked yet"))))

(event `self.Box1.OnComponentEndOverlap`
  (params (OverlappedComponent :type "PrimitiveComponent Object Reference") (OtherActor :type "Actor Object Reference") (OtherComp :type "PrimitiveComponent Object Reference") (OtherBodyIndex :type Integer))
  (bind _asfirst_person_character (cast `/Game/FirstPersonBP/Blueprints/FirstPersonCharacter` OtherActor))
  (set `/Game/FirstPersonBP/Blueprints/FirstPersonCharacter.InElevator?` false _asfirst_person_character)
  (set `/Game/FirstPersonBP/Blueprints/FirstPersonCharacter.ElevatorUp?` (`self.Elevator Down?`) _asfirst_person_character))

(fn `UserConstructionScript`
  (bind _box1 (`self.Box1`))
  ;[1 1 1] Event Begin Play
  (`StaticMeshComponent.SetStaticMesh` (`self.DoorL`) (`self.DoorLMesh`))
  (`StaticMeshComponent.SetStaticMesh` (`self.DoorR`) (`self.DoorRMesh`))
  (if (`self.DoubleDoor?`)
    (`SceneComponent.SetVisibility` (`self.DoorR`) true false)
    (`SceneComponent.SetRelativeScale3D` _box1 (`self.Box Scale`))
    (`SceneComponent.K2_SetRelativeLocation` _box1 (`self.Box Location`) false false)))