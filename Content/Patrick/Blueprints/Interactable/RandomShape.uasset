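; RandomShape is a Blueprint that gives itself a random colour and shape when play begins.
; It picks one of six colour materials at random and applies it to the Shape, CornerCurved and Cylinder components.
; It then makes one randomly chosen component of those three visible, without propagating to children and without hiding the others.
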(event `self.ReceiveBeginPlay`
  (`|ExecutionSequence`
    (:`then_0`
      (for (_array_element _array_index) (`|MakeArray` (`KismetArrayLibrary.Array_Random` (`|MakeArray` "/Game/Materials/Colour_Mat/Material_Colour_Blue2.Material_Colour_Blue2" "/Game/Materials/Colour_Mat/Material_Colour_Green1.Material_Colour_Green1" "/Game/Materials/Colour_Mat/Material_Colour_Orange.Material_Colour_Orange" "/Game/Materials/Colour_Mat/Material_Colour_Purple.Material_Colour_Purple" "/Game/Materials/Colour_Mat/Material_Colour_Red.Material_Colour_Red" "/Game/Materials/Colour_Mat/Material_Colour_Yellow.Material_Colour_Yellow" :!type "MaterialInterface Object Reference")))
        (`PrimitiveComponent.SetMaterial` (`self.Shape`) _array_index _array_element)
        (`PrimitiveComponent.SetMaterial` (`self.CornerCurved`) _array_index _array_element)
        (`PrimitiveComponent.SetMaterial` (`self.Cylinder`) _array_index _array_element)))
    (:`then_1`
      (for _array_element_2 (`|MakeArray` (`KismetArrayLibrary.Array_Random` (`|MakeArray` (`self.Shape`) (`self.CornerCurved`) (`self.Cylinder`) :!type "SceneComponent Object Reference")))
        (`SceneComponent.SetVisibility` _array_element_2 true false)))))

(fn `UserConstructionScript`)