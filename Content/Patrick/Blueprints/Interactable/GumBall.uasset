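; GumBall is an interactable gumball pickup that the first-person character eats to count it and possibly regain stamina.
; It caches the player character on BeginPlay.
; GumballEaten increments the player's gumball count, removes the sphere component and plays a chewing sound.
; Only when stamina is at or below a low threshold does it add stamina and destroy the actor; otherwise the actor remains without its sphere.
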(event `self.ReceiveBeginPlay`
  (bind _asfirst_person_character (cast `/Game/FirstPersonBP/Blueprints/FirstPersonCharacter` (`GameplayStatics.GetPlayerCharacter` 0)))
  (set `self.FPC` _asfirst_person_character))

(event `Gumball Eaten`
  (bind _fpc (`self.FPC`))
  (bind _stamina (`/Game/FirstPersonBP/Blueprints/FirstPersonCharacter.Stamina` _fpc))
  (set `/Game/FirstPersonBP/Blueprints/FirstPersonCharacter.Gumball` (+ (`/Game/FirstPersonBP/Blueprints/FirstPersonCharacter.Gumball` _fpc) 1) _fpc)
  (`ActorComponent.K2_DestroyComponent` (`self.Sphere`))
  (`GameplayStatics.PlaySound2D` "/Game/sounds/ChewingGumball.ChewingGumball" 1.0 1.0 0.0 null null)
  (if (<= _stamina 10.0)
    (set `/Game/FirstPersonBP/Blueprints/FirstPersonCharacter.Stamina` (+ _stamina 10.0) _fpc)
    (`self.K2_DestroyActor`)))

(fn `UserConstructionScript`)