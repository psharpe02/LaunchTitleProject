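; Elevator lift actor that moves its platform up and down in response to the first-person character entering or leaving a trigger box.
; On overlap, the character's InElevator and ElevatorUp flags choose whether a height timeline plays or reverses after a short delay, setting the lift's relative location.
; Leaving the box clears InElevator and drives the timeline in the opposite direction for the same ElevatorUp state.
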(event `self.Box2.OnComponentBeginOverlap`
  (params (OverlappedComponent :type "PrimitiveComponent Object Reference") (OtherActor :type "Actor Object Reference") (OtherComp :type "PrimitiveComponent Object Reference") (OtherBodyIndex :type Integer) (bFromSweep :type Boolean) (SweepResult :type "HitResult Structure (by ref)"))
  ;[1 1 1] Elevator Lift Script
  (bind _asfirst_person_character (cast `/Game/FirstPersonBP/Blueprints/FirstPersonCharacter` OtherActor))
  (if (`/Game/FirstPersonBP/Blueprints/FirstPersonCharacter.InElevator?` _asfirst_person_character)
    (if (`/Game/FirstPersonBP/Blueprints/FirstPersonCharacter.ElevatorUp?` _asfirst_person_character)
      (`KismetSystemLibrary.Delay` 2.0 :!label _label)
      (bind (_direction _height) (`Timeline|ElevatorTL` :!via `Reverse` :!label _label_2)
        (:`Update`
          (`SceneComponent.K2_SetRelativeLocation` (`self.ElevatorLift`) _height false false)))
      (else
        (`KismetSystemLibrary.Delay` 2.0 :!label _label_3)
        (goto _label_2)))))

(event `self.Box2.OnComponentEndOverlap`
  (params (OverlappedComponent :type "PrimitiveComponent Object Reference") (OtherActor :type "Actor Object Reference") (OtherComp :type "PrimitiveComponent Object Reference") (OtherBodyIndex :type Integer))
  ;[1 1 1] Elevator Lift Script
  (bind _asfirst_person_character (cast `/Game/FirstPersonBP/Blueprints/FirstPersonCharacter` OtherActor))
  (set `/Game/FirstPersonBP/Blueprints/FirstPersonCharacter.InElevator?` false _asfirst_person_character)
  (if (`/Game/FirstPersonBP/Blueprints/FirstPersonCharacter.ElevatorUp?` _asfirst_person_character)
    (goto _label_3)
    (else
      (goto _label))))

(fn `UserConstructionScript`)