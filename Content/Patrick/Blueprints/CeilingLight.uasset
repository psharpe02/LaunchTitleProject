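; Configurable ceiling light actor whose LightSwitch enum selects on, off, looping flicker, or a flicker triggered by proximity.
; BeginPlay runs the on, off and delayed loop macros, each acting only in its own mode.
; Player or NPC overlap with the Sphere runs the flicker-off and flicker-on timelines, animating IES brightness.
; The construction script applies spotlight settings and colour presets with matching materials; Tick reapplies the colour every frame.
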(event `LightOff`
  ;[1 1 1] LightSwitch
  (if (`|EnumEquality` (`self.LightSwitch`) "NewEnumerator1")
    (`SceneComponent.SetVisibility` (`self.SpotLight`) false false)))

(event `self.ReceiveBeginPlay`
  (bind _returnvalue (`KismetMathLibrary.RandomFloatInRange` 2.0 10.0))
  ;[1 1 1] LightSwitch
  (`|ExecutionSequence`
    (:`then_0`
      (`self.LightOn`))
    (:`then_1`
      (`self.LightOff`))
    (:`then_2`
      (`KismetSystemLibrary.Delay` _returnvalue)
      (`self.FlickeringLoop` _returnvalue))))

(event `LightOn`
  ;[1 1 1] LightSwitch
  (if (`|EnumEquality` (`self.LightSwitch`) "NewEnumerator0")
    (`SceneComponent.SetVisibility` (`self.SpotLight`) true false)))

(event `LightFlickerOff`
  ;[1 1 1] LightSwitch
  (if (`|EnumEquality` (`self.LightSwitch`) "NewEnumerator6")
    (bind (_direction _value) (`Timeline|FlickerOff`)
      (:`Update`
        (`LightComponent.SetIESBrightnessScale` (`self.SpotLight`) _value))
      (:`Finished`
        (`PrimitiveComponent.SetMaterial` (`self.Light`) 1 "/Game/Models/James/RectangleLights/base.base")))))

(event `LightFlickerOn`
  (bind _spotlight (`self.SpotLight`))
  ;[1 1 1] LightSwitch
  (if (`|EnumEquality` (`self.LightSwitch`) "NewEnumerator5")
    (`PrimitiveComponent.SetMaterial` (`self.Light`) 1 "/Game/Models/James/RectangleLights/base.base")
    (`LightComponent.SetIESBrightnessScale` (`self.SpotLight`) 0.0)
    (bind (_direction _value) (`Timeline|FlickerOn`)
      (:`Update`
        (`LightComponent.SetIESBrightnessScale` _spotlight _value)
        (`KismetSystemLibrary.Delay` 5.0)
        (`PrimitiveComponent.SetMaterial` (`self.Light`) 1 "/Game/Models/James/RectangleLights/Light.Light"))
      (:`Finished`
        (`SceneComponent.SetVisibility` _spotlight false false)))))

(event `self.Sphere.OnComponentBeginOverlap`
  (params (OverlappedComponent :type "PrimitiveComponent Object Reference") (OtherActor :type "Actor Object Reference") (OtherComp :type "PrimitiveComponent Object Reference") (OtherBodyIndex :type Integer) (bFromSweep :type Boolean) (SweepResult :type "HitResult Structure (by ref)"))
  ;[1 1 1] LightSwitch
  (`|ExecutionSequence`
    (:`then_0`
      (cast `/Game/FirstPersonBP/Blueprints/FirstPersonCharacter` OtherActor))
    (:`then_1`
      (cast `/Game/Turlough/AI/Bear_AI/NPC` OtherActor)))
  (`|ExecutionSequence`
    (:`then_0`
      (`self.LightFlickerOff`))
    (:`then_1`
      (`self.LightFlickerOn`))))

(event `FlickeringLoop`
  (params (NewTime :type "Float (double-precision)"))
  ;[1 1 1] LightSwitch
  (if (`|EnumEquality` (`self.LightSwitch`) "NewEnumerator2")
    (if (`self.Faster Light?`)
      (bind (_direction _value) (`Timeline|Timeline_2`)
        (:`Update`
          (`LightComponent.SetIESBrightnessScale` (`self.SpotLight`) _value)))
      (else
        (bind (_direction_2 _value_2) (`Timeline|Timeline_1` :`NewTime` NewTime)
          (:`Update`
            (`LightComponent.SetIESBrightnessScale` (`self.SpotLight`) _value_2)))))))

(event `self.ReceiveTick`
  (params (DeltaSeconds :type "Float (single-precision)"))
  (bind _lightcolours (`self.LightColours`))
  (bind _spotlight (`self.SpotLight`))
  ;[1 1 1] Light Colours
  (`|ExecutionSequence`
    (:`then_0`
      (if (`|EnumEquality` _lightcolours "NewEnumerator6")
        (bind _output_get (set `self.Light Color` (struct :`R` 1.0 :`G` 1.0 :`B` 0.799103 :`A` 1.0)))
        (`LightComponent.SetLightColor` _spotlight _output_get true)
        (`PrimitiveComponent.SetMaterial` (`self.Light`) (`self.Element Index`) "/Game/Models/James/RectangleLights/Light.Light")))
    (:`then_1`
      (if (`|EnumEquality` _lightcolours "NewEnumerator1")
        (bind _output_get_2 (set `self.Light Color` (struct :`R` 0.379167 :`G` 0.049371 :`B` 0.06122 :`A` 1.0)))
        (`LightComponent.SetLightColor` _spotlight _output_get_2 true)
        (`PrimitiveComponent.SetMaterial` (`self.Light`) (`self.Element Index`) "/Game/Materials/Colour_Mat/Material_Colour_Red.Material_Colour_Red")))
    (:`then_2`
      (if (`|EnumEquality` _lightcolours "NewEnumerator0")
        (bind _output_get_3 (set `self.Light Color` (struct :`R` 0.060364 :`G` 0.379167 :`B` 0.049371 :`A` 1.0)))
        (`LightComponent.SetLightColor` _spotlight _output_get_3 true)
        (`PrimitiveComponent.SetMaterial` (`self.Light`) (`self.Element Index`) "/Game/Materials/Colour_Mat/Material_Colour_Green1.Material_Colour_Green1")))
    (:`then_3`
      (if (`|EnumEquality` _lightcolours "NewEnumerator5")
        (bind _output_get_4 (set `self.Light Color` (struct :`R` 0.049371 :`G` 0.126323 :`B` 0.379167 :`A` 1.0)))
        (`LightComponent.SetLightColor` _spotlight _output_get_4 true)
        (`PrimitiveComponent.SetMaterial` (`self.Light`) (`self.Element Index`) "/Game/Materials/Colour_Mat/Material_Colour_Blue2.Material_Colour_Blue2")))
    (:`then_4`
      (if (`|EnumEquality` _lightcolours "NewEnumerator2")
        (bind _output_get_5 (set `self.Light Color` (struct :`R` 0.379167 :`G` 0.368174 :`B` 0.049371 :`A` 1.0)))
        (`LightComponent.SetLightColor` _spotlight _output_get_5 true)
        (`PrimitiveComponent.SetMaterial` (`self.Light`) (`self.Element Index`) "/Game/Materials/Colour_Mat/Material_Colour_Yellow.Material_Colour_Yellow")))))

(event `Light Custom`
  (params (`Point Light` :type "LightComponent Object Reference") (`Spot Light` :type "LightComponent Object Reference") (`Spot Light Scene` :type "SceneComponent Object Reference") (`Local Spot Light` :type "LocalLightComponent Object Reference") (`PointLight Intensity` :type "Float (double-precision)") (`Attenuation Radius` :type "Float (double-precision)") (`IES Texture` :type "TextureLightProfile Object Reference") (`IES Intensity` :type "Float (double-precision)") (`Spot Light Location` :type "Vector Structure") (`Spot Light Rotation` :type "Rotator Structure") (ElementIndex :type Integer) (Material :type "MaterialInterface Object Reference") (OuterConeAngle :type "Float (double-precision)") (InnerConeAngle :type "Float (double-precision)"))
  (bind _spotlight (`self.SpotLight`))
  ;[1 1 1] Light Custom
  (`LightComponent.SetIntensity` `Point Light` `PointLight Intensity`)
  (`LocalLightComponent.SetAttenuationRadius` `Local Spot Light` `Attenuation Radius`)
  (`LightComponent.SetIESTexture` `Spot Light` `IES Texture`)
  (`LightComponent.SetIESBrightnessScale` `Spot Light` (* `IES Intensity` (`self.Light Multiplier`)))
  (`SceneComponent.K2_SetRelativeLocationAndRotation` `Spot Light Scene` `Spot Light Location` `Spot Light Rotation` false false)
  (`PrimitiveComponent.SetMaterial` (`self.Light`) ElementIndex Material)
  (`SpotLightComponent.SetOuterConeAngle` _spotlight OuterConeAngle)
  (`SpotLightComponent.SetInnerConeAngle` _spotlight InnerConeAngle))

(fn `UserConstructionScript`
  (bind _spotlight (`self.SpotLight`))
  (bind _lightcolours (`self.LightColours`))
  (bind _spotlight_2 (`self.SpotLight`))
  (`|ExecutionSequence`
    (:`then_0`
      (`SceneComponent.K2_SetWorldLocation` (`self.Sphere`) (+ (`SceneComponent.RelativeLocation` (`self.DefaultSceneRoot`)) (`self.Player Collision`)) false false))
    (:`then_1`
      ;[1 1 1] Light Colours
      (`|ExecutionSequence`
        (:`then_0`
          (if (`|EnumEquality` _lightcolours "NewEnumerator6")
            (bind _output_get (set `self.Light Color` (struct :`R` 1.0 :`G` 1.0 :`B` 0.799103 :`A` 1.0)))
            (`LightComponent.SetLightColor` _spotlight_2 _output_get true)
            (`PrimitiveComponent.SetMaterial` (`self.Light`) (`self.Element Index`) "/Game/Models/James/RectangleLights/Light.Light")))
        (:`then_1`
          (if (`|EnumEquality` _lightcolours "NewEnumerator1")
            (bind _output_get_2 (set `self.Light Color` (struct :`R` 0.379167 :`G` 0.049371 :`B` 0.06122 :`A` 1.0)))
            (`LightComponent.SetLightColor` _spotlight_2 _output_get_2 true)
            (`PrimitiveComponent.SetMaterial` (`self.Light`) (`self.Element Index`) "/Game/Materials/Colour_Mat/Material_Colour_Red.Material_Colour_Red")))
        (:`then_2`
          (if (`|EnumEquality` _lightcolours "NewEnumerator0")
            (bind _output_get_3 (set `self.Light Color` (struct :`R` 0.060364 :`G` 0.379167 :`B` 0.049371 :`A` 1.0)))
            (`LightComponent.SetLightColor` _spotlight_2 _output_get_3 true)
            (`PrimitiveComponent.SetMaterial` (`self.Light`) (`self.Element Index`) "/Game/Materials/Colour_Mat/Material_Colour_Green1.Material_Colour_Green1")))
        (:`then_3`
          (if (`|EnumEquality` _lightcolours "NewEnumerator5")
            (bind _output_get_4 (set `self.Light Color` (struct :`R` 0.049371 :`G` 0.126323 :`B` 0.379167 :`A` 1.0)))
            (`LightComponent.SetLightColor` _spotlight_2 _output_get_4 true)
            (`PrimitiveComponent.SetMaterial` (`self.Light`) (`self.Element Index`) "/Game/Materials/Colour_Mat/Material_Colour_Blue2.Material_Colour_Blue2")))
        (:`then_4`
          (if (`|EnumEquality` _lightcolours "NewEnumerator2")
            (bind _output_get_5 (set `self.Light Color` (struct :`R` 0.379167 :`G` 0.368174 :`B` 0.049371 :`A` 1.0)))
            (`LightComponent.SetLightColor` _spotlight_2 _output_get_5 true)
            (`PrimitiveComponent.SetMaterial` (`self.Light`) (`self.Element Index`) "/Game/Materials/Colour_Mat/Material_Colour_Yellow.Material_Colour_Yellow")))))
    (:`then_2`
      (`self.Light Custom` _spotlight _spotlight _spotlight _spotlight (`self.PointLight Intensity`) (`self.Attenuation Radius`) (`self.IES Texture`) (`self.IES Intensity`) (`self.Spot Light Location`) (`self.Spot Light Rotation`) (`self.Element Index`) (`self.Material`) (`self.Outer Cone Angle`) (`self.Inner Cone Angle`)))))