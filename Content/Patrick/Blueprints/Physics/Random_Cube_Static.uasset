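; Random_Cube_Static is a cube actor that randomises its look on BeginPlay.
; A sequence gives the Cube mesh a random colour material from six, then one of four uniform scales at its current relative location.
; Each random pick passes through a one-element ForEach loop.
; The transform's rotation reads a third random-rotator loop that runs afterwards with an empty body, so the random rotation is not yet set when applied.
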(event `self.ReceiveBeginPlay`
  (bind _cube (`self.Cube`))
  (`|ExecutionSequence`
    (:`then_0`
      (for (_array_element _array_index) (`|MakeArray` (`KismetArrayLibrary.Array_Random` (`|MakeArray` "/Game/Materials/Colour_Mat/Material_Colour_Blue2.Material_Colour_Blue2" "/Game/Materials/Colour_Mat/Material_Colour_Green1.Material_Colour_Green1" "/Game/Materials/Colour_Mat/Material_Colour_Orange.Material_Colour_Orange" "/Game/Materials/Colour_Mat/Material_Colour_Purple.Material_Colour_Purple" "/Game/Materials/Colour_Mat/Material_Colour_Red.Material_Colour_Red" "/Game/Materials/Colour_Mat/Material_Colour_Yellow.Material_Colour_Yellow" :!type "MaterialInterface Object Reference")))
        (`PrimitiveComponent.SetMaterial` (`self.Cube`) _array_index _array_element)))
    (:`then_1`
      (for _array_element_2 (`|MakeArray` (`KismetArrayLibrary.Array_Random` (`|MakeArray` (0.4 0.4 0.4) (0.3 0.3 0.3) (0.5 0.5 0.5) (0.6 0.6 0.6) :!type "Vector Structure")))
        (`SceneComponent.K2_SetRelativeTransform` _cube (`KismetMathLibrary.MakeTransform` (`SceneComponent.RelativeLocation` _cube) (stale _array_element_3) _array_element_2) false false)))
    (:`then_2`
      (for _array_element_3 (`|MakeArray` (`KismetArrayLibrary.Array_Random` (`|MakeArray` (`KismetMathLibrary.RandomRotator` false) (`KismetMathLibrary.RandomRotator` false) (`KismetMathLibrary.RandomRotator` false) (`KismetMathLibrary.RandomRotator` false))))
        _))))

(fn `UserConstructionScript`)