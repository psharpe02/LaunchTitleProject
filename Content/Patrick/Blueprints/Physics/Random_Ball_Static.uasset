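; Ball-pit ball actor that randomises its look when play begins.
; BeginPlay picks one of six colour materials at random and applies it to the BallBallpit component's first material slot.
; It then picks one of four uniform scales at random, keeping the component's relative location and rotation.
; Both picks run at runtime, as the construction script is empty.
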(event `self.ReceiveBeginPlay`
  (bind _ball_ballpit (`self.ball_ballpit`))
  (`|ExecutionSequence`
    (:`then_0`
      (for (_array_element _array_index) (`|MakeArray` (`KismetArrayLibrary.Array_Random` (`|MakeArray` "/Game/Materials/Colour_Mat/Material_Colour_Blue2.Material_Colour_Blue2" "/Game/Materials/Colour_Mat/Material_Colour_Green1.Material_Colour_Green1" "/Game/Materials/Colour_Mat/Material_Colour_Orange.Material_Colour_Orange" "/Game/Materials/Colour_Mat/Material_Colour_Purple.Material_Colour_Purple" "/Game/Materials/Colour_Mat/Material_Colour_Red.Material_Colour_Red" "/Game/Materials/Colour_Mat/Material_Colour_Yellow.Material_Colour_Yellow" :!type "MaterialInterface Object Reference")))
        (`PrimitiveComponent.SetMaterial` (`self.ball_ballpit`) _array_index _array_element)))
    (:`then_1`
      (for _array_element_2 (`|MakeArray` (`KismetArrayLibrary.Array_Random` (`|MakeArray` (20.0 20.0 20.0) (15.0 15.0 15.0) (25.0 25.0 25.0) (35.0 35.0 35.0) :!type "Vector Structure")))
        (`SceneComponent.K2_SetRelativeTransform` _ball_ballpit (`KismetMathLibrary.MakeTransform` (`SceneComponent.RelativeLocation` _ball_ballpit) (`SceneComponent.RelativeRotation` _ball_ballpit) _array_element_2) false false)))))

(fn `UserConstructionScript`)