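; Blueprint that displays a configurable static mesh with a randomly chosen material.
; It sets ModelMesh on the Model component and applies a random entry from the Material array to slot 0.
; The same logic runs in the construction script and again on BeginPlay, so the material is re-rolled when play starts.
; Each pass wraps the single random pick in a one-element loop.
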(event `self.ReceiveBeginPlay`
  (bind _model (`self.Model`))
  (for _array_element (`|MakeArray` (`KismetArrayLibrary.Array_Random` (`self.Material`)))
    (`StaticMeshComponent.SetStaticMesh` _model (`self.ModelMesh`))
    (`PrimitiveComponent.SetMaterial` _model 0 _array_element)))

(fn `UserConstructionScript`
  (bind _model (`self.Model`))
  (for _array_element (`|MakeArray` (`KismetArrayLibrary.Array_Random` (`self.Material`)))
    (`StaticMeshComponent.SetStaticMesh` _model (`self.ModelMesh`))
    (`PrimitiveComponent.SetMaterial` _model 0 _array_element)))