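; MusicBox is a music trigger that plays a sound when the FirstPersonCharacter overlaps its Box.
; Begin overlap spawns the sound on a new audio component through a DoOnce gated by SongFinished, which clears if playback starts.
; End overlap stops the sound and sets SongFinished.
; The DoOnce resets only on a begin overlap while SongFinished is false, so simply leaving and re-entering does not replay it.
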(event `self.Box.OnComponentBeginOverlap`
  (params (OverlappedComponent :type "PrimitiveComponent Object Reference") (OtherActor :type "Actor Object Reference") (OtherComp :type "PrimitiveComponent Object Reference") (OtherBodyIndex :type Integer) (bFromSweep :type Boolean) (SweepResult :type "HitResult Structure (by ref)"))
  (cast `/Game/FirstPersonBP/Blueprints/FirstPersonCharacter` OtherActor)
  (if (`self.SongFinished?`)
    (`/Engine/EditorBlueprintResources/StandardMacros.DoOnce` false :!label _label
      (:`Completed`
        (bind _returnvalue (`AddComponent|NODE_AddAudioComponent-1`))
        (bind _returnvalue_2 (`GameplayStatics.SpawnSoundAttached` (`self.New Sound`) _returnvalue "None" (0.0 0.0 0.0) (struct) "KeepRelativeOffset" false 1.0 1.0 0.0 null null))
        (if (`AudioComponent.IsPlaying` _returnvalue_2)
          (set `self.SongFinished?` false))))
    (else
      (goto _label :!via `Reset`))))

(event `self.Box.OnComponentEndOverlap`
  (params (OverlappedComponent :type "PrimitiveComponent Object Reference") (OtherActor :type "Actor Object Reference") (OtherComp :type "PrimitiveComponent Object Reference") (OtherBodyIndex :type Integer))
  (cast `/Game/FirstPersonBP/Blueprints/FirstPersonCharacter` OtherActor)
  (set `self.SongFinished?` true)
  (`/Engine/EditorBlueprintResources/StandardMacros.IsValid` (stale `self.Box.OnComponentBeginOverlap` _returnvalue_2)
    (:`Is Valid`
      (`AudioComponent.Stop` (stale `self.Box.OnComponentBeginOverlap` _returnvalue_2)))))

(fn `UserConstructionScript`)