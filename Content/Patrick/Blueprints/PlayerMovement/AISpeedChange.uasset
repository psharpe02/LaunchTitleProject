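; AISpeedChange is a trigger volume that changes NPC speed through the AI blackboard.
; When an NPC enters the Box, it sets the Activation key to true and lowers the VentSpeed value.
; When the NPC leaves, it raises VentSpeed again but leaves Activation set.
; The Blueprint only writes blackboard keys, so applying the speed happens outside this file.
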(event `self.Box.OnComponentBeginOverlap`
  (params (OverlappedComponent :type "PrimitiveComponent Object Reference") (OtherActor :type "Actor Object Reference") (OtherComp :type "PrimitiveComponent Object Reference") (OtherBodyIndex :type Integer) (bFromSweep :type Boolean) (SweepResult :type "HitResult Structure (by ref)"))
  (bind _asnpc (cast `/Game/Turlough/AI/Bear_AI/NPC` OtherActor))
  (bind _returnvalue (`AIBlueprintHelperLibrary.GetBlackboard` _asnpc))
  (`BlackboardComponent.SetValueAsBool` _returnvalue "Activation" true)
  (`BlackboardComponent.SetValueAsFloat` _returnvalue "VentSpeed" 100.0))

(event `self.Box.OnComponentEndOverlap`
  (params (OverlappedComponent :type "PrimitiveComponent Object Reference") (OtherActor :type "Actor Object Reference") (OtherComp :type "PrimitiveComponent Object Reference") (OtherBodyIndex :type Integer))
  (bind _asnpc (cast `/Game/Turlough/AI/Bear_AI/NPC` OtherActor))
  (`BlackboardComponent.SetValueAsFloat` (`AIBlueprintHelperLibrary.GetBlackboard` _asnpc) "VentSpeed" 250.0))

(fn `UserConstructionScript`)