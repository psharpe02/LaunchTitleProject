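; SlippyFloor is a floor volume that changes the first-person character's braking to make it slippery.
; When the character enters the Box, two timelines drive its CharacterMovement braking friction factor and walking braking deceleration over time.
; Leaving the Box sets both properties back to hardcoded values rather than cached originals, without stopping the timelines.
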(event `self.ReceiveBeginPlay`)

(event `self.Box.OnComponentBeginOverlap`
  (params (OverlappedComponent :type "PrimitiveComponent Object Reference") (OtherActor :type "Actor Object Reference") (OtherComp :type "PrimitiveComponent Object Reference") (OtherBodyIndex :type Integer) (bFromSweep :type Boolean) (SweepResult :type "HitResult Structure (by ref)"))
  (bind _asfirst_person_character (cast `/Game/FirstPersonBP/Blueprints/FirstPersonCharacter` OtherActor))
  (bind _charactermovement (`Character.CharacterMovement` _asfirst_person_character))
  (`/Engine/EditorBlueprintResources/StandardMacros.IsValid` _charactermovement
    (:`Is Valid`
      (`|ExecutionSequence`
        (:`then_0`
          (bind (_direction _value) (`Timeline|Braking Friction` :`NewTime` (`CharacterMovementComponent.BrakingFrictionFactor` _charactermovement))
            (:`Update`
              (set `CharacterMovementComponent.BrakingFrictionFactor` _value _charactermovement))))
        (:`then_1`
          (bind (_direction_2 _value_2) (`Timeline|Braking Deceleration` :`NewTime` (`CharacterMovementComponent.BrakingDecelerationWalking` _charactermovement))
            (:`Update`
              (set `CharacterMovementComponent.BrakingDecelerationWalking` _value_2 _charactermovement))))))))

(event `self.Box.OnComponentEndOverlap`
  (params (OverlappedComponent :type "PrimitiveComponent Object Reference") (OtherActor :type "Actor Object Reference") (OtherComp :type "PrimitiveComponent Object Reference") (OtherBodyIndex :type Integer))
  (bind _asfirst_person_character (cast `/Game/FirstPersonBP/Blueprints/FirstPersonCharacter` OtherActor))
  (bind _charactermovement (`Character.CharacterMovement` _asfirst_person_character))
  (`/Engine/EditorBlueprintResources/StandardMacros.IsValid` _charactermovement
    (:`Is Valid`
      (set `CharacterMovementComponent.BrakingFrictionFactor` 2.0 _charactermovement)
      (set `CharacterMovementComponent.BrakingDecelerationWalking` 2048.0 _charactermovement))))

(fn `UserConstructionScript`)