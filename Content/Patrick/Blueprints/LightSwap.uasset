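; Configurable light fixture actor with selectable mesh type, colour and switch behaviour: on, off, or flickering.
; The construction script sets the mesh, light settings and colour preset, and Tick reapplies the colour every frame.
; BeginPlay applies on or off states and starts FlickeringLoop after a random delay, while FirstPersonCharacter overlapping the sphere triggers flicker-off or flicker-on.
; Each LightSwitch-gated node changes visibility or material, with timelines animating IES brightness for flickers.
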(event `self.ReceiveBeginPlay`
  (`|ExecutionSequence`
    (:`then_1`
      ;[1 1 1] LightSwitch
      (`|ExecutionSequence`
        (:`then_0`
          (`self.LightOn`))
        (:`then_1`
          (`self.LightOff`))
        (:`then_2`
          (`KismetSystemLibrary.Delay` (`KismetMathLibrary.RandomFloatInRange` 2.0 10.0))
          (`self.FlickeringLoop`))))))

(event `LightOff`
  ;[1 1 1] LightSwitch
  (if (`|EnumEquality` (`self.LightSwitch`) "NewEnumerator1")
    (`SceneComponent.SetVisibility` (`self.PointLight`) false false)
    (`SceneComponent.SetVisibility` (`self.SpotLight`) false false)
    (`PrimitiveComponent.SetMaterial` (`self.Light`) 1 "/Game/Models/James/base.base")))

(event `self.Sphere.OnComponentBeginOverlap`
  (params (OverlappedComponent :type "PrimitiveComponent Object Reference") (OtherActor :type "Actor Object Reference") (OtherComp :type "PrimitiveComponent Object Reference") (OtherBodyIndex :type Integer) (bFromSweep :type Boolean) (SweepResult :type "HitResult Structure (by ref)"))
  ;[1 1 1] LightSwitch
  (cast `/Game/FirstPersonBP/Blueprints/FirstPersonCharacter` OtherActor)
  (`|ExecutionSequence`
    (:`then_0`
      (`self.LightFlickerOff`))
    (:`then_1`
      (`self.LightFlickerOn`))))

(event `LightOn`
  ;[1 1 1] LightSwitch
  (if (`|EnumEquality` (`self.LightSwitch`) "NewEnumerator0")
    (`SceneComponent.SetVisibility` (`self.PointLight`) true false)
    (`SceneComponent.SetVisibility` (`self.SpotLight`) true false)))

(event `LightFlickerOff`
  ;[1 1 1] LightSwitch
  (if (`|EnumEquality` (`self.LightSwitch`) "NewEnumerator6")
    (bind (_direction _value) (`Timeline|FlickerOff`)
      (:`Update`
        (`LightComponent.SetIESBrightnessScale` (`self.SpotLight`) _value))
      (:`Finished`
        (`SceneComponent.SetVisibility` (`self.PointLight`) false false)
        (`SceneComponent.SetVisibility` (`self.SpotLight`) false false)
        (`PrimitiveComponent.SetMaterial` (`self.Light`) 1 "/Game/Models/James/base.base")))))

(event `LightFlickerOn`
  ;[1 1 1] LightSwitch
  (if (`|EnumEquality` (`self.LightSwitch`) "NewEnumerator5")
    (`PrimitiveComponent.SetMaterial` (`self.Light`) 1 "/Game/Models/James/base.base")
    (`LightComponent.SetIESBrightnessScale` (`self.SpotLight`) 0.0)
    (`LightComponent.SetIESBrightnessScale` (`self.PointLight`) 0.0)
    (bind (_direction _value) (`Timeline|FlickerOn`)
      (:`Update`
        (`LightComponent.SetIESBrightnessScale` (`self.SpotLight`) _value)
        (`KismetSystemLibrary.Delay` 5.0)
        (`PrimitiveComponent.SetMaterial` (`self.Light`) 1 "/Game/Models/James/Light.Light"))
      (:`Finished`
        (`SceneComponent.SetVisibility` (`self.PointLight`) true false)
        (`SceneComponent.SetVisibility` (`self.SpotLight`) true false)))))

(event `FlickeringLoop`
  ;[1 1 1] LightSwitch
  (if (`|EnumEquality` (`self.LightSwitch`) "NewEnumerator2")
    (bind (_direction _value) (`Timeline|FlickerLoop`)
      (:`Update`
        (`LightComponent.SetIESBrightnessScale` (`self.SpotLight`) _value))
      (:`Finished`
        (`SceneComponent.SetVisibility` (`self.PointLight`) false false)
        (`SceneComponent.SetVisibility` (`self.SpotLight`) false false)
        (`PrimitiveComponent.SetMaterial` (`self.Light`) 1 "/Game/Models/James/base.base")))))

(event `self.ReceiveTick`
  (params (DeltaSeconds :type "Float (single-precision)"))
  (bind _lightcolours (`self.LightColours`))
  (bind _spotlight (`self.SpotLight`))
  ;[1 1 1] Light Colours
  (`|ExecutionSequence`
    (:`then_0`
      (if (`|EnumEquality` _lightcolours "NewEnumerator6")
        (bind _output_get (set `self.Light Color` (struct :`R` 1.0 :`G` 1.0 :`B` 0.799103 :`A` 1.0)))
        (`LightComponent.SetLightColor` _spotlight _output_get true)
        (`LightComponent.SetLightColor` (`self.PointLight`) _output_get true)
        (`PrimitiveComponent.SetMaterial` (`self.Light`) (`self.Element Index`) "/Game/Models/James/Light.Light")))
    (:`then_1`
      (if (`|EnumEquality` _lightcolours "NewEnumerator1")
        (bind _output_get_2 (set `self.Light Color` (struct :`R` 0.379167 :`G` 0.049371 :`B` 0.06122 :`A` 1.0)))
        (`LightComponent.SetLightColor` _spotlight _output_get_2 true)
        (`LightComponent.SetLightColor` (`self.PointLight`) _output_get_2 true)
        (`PrimitiveComponent.SetMaterial` (`self.Light`) (`self.Element Index`) "/Game/Materials/Colour_Mat/Material_Colour_Red.Material_Colour_Red")))
    (:`then_2`
      (if (`|EnumEquality` _lightcolours "NewEnumerator0")
        (bind _output_get_3 (set `self.Light Color` (struct :`R` 0.060364 :`G` 0.379167 :`B` 0.049371 :`A` 1.0)))
        (`LightComponent.SetLightColor` _spotlight _output_get_3 true)
        (`LightComponent.SetLightColor` (`self.PointLight`) _output_get_3 true)
        (`PrimitiveComponent.SetMaterial` (`self.Light`) (`self.Element Index`) "/Game/Materials/Colour_Mat/Material_Colour_Green1.Material_Colour_Green1")))
    (:`then_3`
      (if (`|EnumEquality` _lightcolours "NewEnumerator5")
        (bind _output_get_4 (set `self.Light Color` (struct :`R` 0.049371 :`G` 0.126323 :`B` 0.379167 :`A` 1.0)))
        (`LightComponent.SetLightColor` _spotlight _output_get_4 true)
        (`LightComponent.SetLightColor` (`self.PointLight`) _output_get_4 true)
        (`PrimitiveComponent.SetMaterial` (`self.Light`) (`self.Element Index`) "/Game/Materials/Colour_Mat/Material_Colour_Blue2.Material_Colour_Blue2")))
    (:`then_4`
      (if (`|EnumEquality` _lightcolours "NewEnumerator2")
        (bind _output_get_5 (set `self.Light Color` (struct :`R` 0.379167 :`G` 0.368174 :`B` 0.049371 :`A` 1.0)))
        (`LightComponent.SetLightColor` _spotlight _output_get_5 true)
        (`LightComponent.SetLightColor` (`self.PointLight`) _output_get_5 true)
        (`PrimitiveComponent.SetMaterial` (`self.Light`) (`self.Element Index`) "/Game/Materials/Colour_Mat/Material_Colour_Yellow.Material_Colour_Yellow")))))

(fn `Light Custom`
  (params (`Point Light` :type "LightComponent Object Reference") (`Spot Light` :type "LightComponent Object Reference") (`Spot Light Scene` :type "SceneComponent Object Reference") (`Local Spot Light` :type "LocalLightComponent Object Reference") (`PointLight Intensity` :type "Float (double-precision)") (`Attenuation Radius` :type "Float (double-precision)") (`IES Texture` :type "TextureLightProfile Object Reference") (`IES Intensity` :type "Float (double-precision)") (`Spot Light Location` :type "Vector Structure") (`Spot Light Rotation` :type "Rotator Structure") (`Light Actor` :type "PrimitiveComponent Object Reference") (ElementIndex :type Integer) (Material :type "MaterialInterface Object Reference"))
  (`LightComponent.SetIntensity` `Point Light` `PointLight Intensity`)
  (`LocalLightComponent.SetAttenuationRadius` `Local Spot Light` `Attenuation Radius`)
  (`LightComponent.SetIESTexture` `Spot Light` `IES Texture`)
  (`LightComponent.SetIESBrightnessScale` `Spot Light` `IES Intensity`)
  (`SceneComponent.K2_SetRelativeLocationAndRotation` `Spot Light Scene` `Spot Light Location` `Spot Light Rotation` false false)
  (`PrimitiveComponent.SetMaterial` `Light Actor` ElementIndex Material))

(fn `UserConstructionScript`
  (bind _light (`self.Light`))
  (bind _lighttypes (`self.LightTypes`))
  (bind _lightcolours (`self.LightColours`))
  (bind _spotlight (`self.SpotLight`))
  (bind _rectlight (`self.RectLight`))
  (bind _spotlight_2 (`self.SpotLight`))
  (bind _light_2 (`self.Light`))
  (bind _spotlight_3 (`self.SpotLight`))
  (bind _light_3 (`self.Light`))
  (bind (_relativelocation_x _relativelocation_y _relativelocation_z) (`KismetMathLibrary.BreakVector` (`SceneComponent.RelativeLocation` _light)))
  (bind (_relativerotation_roll _relativerotation_pitch _relativerotation_yaw) (`KismetMathLibrary.BreakRotator` (`SceneComponent.RelativeRotation` _light_2)))
  (bind (_relativelocation_x_2 _relativelocation_y_2 _relativelocation_z_2) (`KismetMathLibrary.BreakVector` (`SceneComponent.RelativeLocation` _light_2)))
  (`|ExecutionSequence`
    (:`then_0`
      ;[1 1 1] Light Types
      (if (`|EnumEquality` _lighttypes "NewEnumerator0")
        (bind _returnvalue (`StaticMeshComponent.SetStaticMesh` _light_3 "/Game/Models/James/ceiling_light_resized.ceiling_light_resized"))
        (if _returnvalue
          (if (`self.NoCustom?`)
            (`self.Light Custom` _rectlight _rectlight _rectlight _rectlight (`self.PointLight Intensity`) (`self.Attenuation Radius`) (`self.IES Texture`) (`self.IES Intensity`) (`self.Spot Light Location`) (`self.Spot Light Rotation`) (`self.Light`) (`self.Element Index`) (`self.Material`))))
        (elif (`|EnumEquality` _lighttypes "NewEnumerator1")
          (bind _returnvalue_2 (`StaticMeshComponent.SetStaticMesh` _light_3 "/Game/Patrick/Meshes/BlockoutAssets/CircularBlockoutMesh.CircularBlockoutMesh"))
          (if _returnvalue_2
            (`SceneComponent.K2_SetRelativeLocationAndRotation` _light_2 (`KismetMathLibrary.MakeVector` _relativelocation_x_2 _relativelocation_y_2 (+ _relativelocation_z_2 20.0)) (`KismetMathLibrary.MakeRotator` (+ _relativerotation_roll 180.0) _relativerotation_pitch _relativerotation_yaw) false false)
            (`SceneComponent.SetRelativeScale3D` (`self.Light`) (`self.Light Size`))
            (if (`self.NoCustom?`)
              (`self.Light Custom` (`self.PointLight`) _spotlight_3 _spotlight_3 _spotlight_3 (`self.PointLight Intensity`) (`self.Attenuation Radius`) (`self.IES Texture`) (`self.IES Intensity`) (`self.Spot Light Location`) (`self.Spot Light Rotation`) (`self.Light`) (`self.Element Index`) (`self.Material`))))
          (elif (`|EnumEquality` _lighttypes "NewEnumerator2")
            (bind _returnvalue_3 (`StaticMeshComponent.SetStaticMesh` _light_3 "/Game/Patrick/Meshes/BlockoutAssets/NeonLights.NeonLights"))
            (if _returnvalue_3
              (`SceneComponent.K2_SetRelativeLocationAndRotation` _light (`KismetMathLibrary.MakeVector` (+ _relativelocation_x 135.0) _relativelocation_y _relativelocation_z) (`SceneComponent.RelativeRotation` _light) false false)
              (if (`self.NoCustom?`)
                (`self.Light Custom` (`self.PointLight`) _spotlight_2 _spotlight_2 _spotlight_2 (`self.PointLight Intensity`) (`self.Attenuation Radius`) (`self.IES Texture`) (`self.IES Intensity`) (`self.Spot Light Location`) (`self.Spot Light Rotation`) (`self.Light`) (`self.Element Index`) (`self.Material`))))
            (elif (`|EnumEquality` _lighttypes "NewEnumerator3")
              (`StaticMeshComponent.SetStaticMesh` _light_3 "/Game/Models/James/ceiling_light_resized.ceiling_light_resized"))))))
    (:`then_1`
      ;[1 1 1] Light Colours
      (`|ExecutionSequence`
        (:`then_0`
          (if (`|EnumEquality` _lightcolours "NewEnumerator6")
            (bind _output_get (set `self.Light Color` (struct :`R` 1.0 :`G` 1.0 :`B` 0.799103 :`A` 1.0)))
            (`LightComponent.SetLightColor` _spotlight _output_get true)
            (`LightComponent.SetLightColor` (`self.PointLight`) _output_get true)
            (`PrimitiveComponent.SetMaterial` (`self.Light`) (`self.Element Index`) "/Game/Models/James/Light.Light")))
        (:`then_1`
          (if (`|EnumEquality` _lightcolours "NewEnumerator1")
            (bind _output_get_2 (set `self.Light Color` (struct :`R` 0.379167 :`G` 0.049371 :`B` 0.06122 :`A` 1.0)))
            (`LightComponent.SetLightColor` _spotlight _output_get_2 true)
            (`LightComponent.SetLightColor` (`self.PointLight`) _output_get_2 true)
            (`PrimitiveComponent.SetMaterial` (`self.Light`) (`self.Element Index`) "/Game/Materials/Colour_Mat/Material_Colour_Red.Material_Colour_Red")))
        (:`then_2`
          (if (`|EnumEquality` _lightcolours "NewEnumerator0")
            (bind _output_get_3 (set `self.Light Color` (struct :`R` 0.060364 :`G` 0.379167 :`B` 0.049371 :`A` 1.0)))
            (`LightComponent.SetLightColor` _spotlight _output_get_3 true)
            (`LightComponent.SetLightColor` (`self.PointLight`) _output_get_3 true)
            (`PrimitiveComponent.SetMaterial` (`self.Light`) (`self.Element Index`) "/Game/Materials/Colour_Mat/Material_Colour_Green1.Material_Colour_Green1")))
        (:`then_3`
          (if (`|EnumEquality` _lightcolours "NewEnumerator5")
            (bind _output_get_4 (set `self.Light Color` (struct :`R` 0.049371 :`G` 0.126323 :`B` 0.379167 :`A` 1.0)))
            (`LightComponent.SetLightColor` _spotlight _output_get_4 true)
            (`LightComponent.SetLightColor` (`self.PointLight`) _output_get_4 true)
            (`PrimitiveComponent.SetMaterial` (`self.Light`) (`self.Element Index`) "/Game/Materials/Colour_Mat/Material_Colour_Blue2.Material_Colour_Blue2")))
        (:`then_4`
          (if (`|EnumEquality` _lightcolours "NewEnumerator2")
            (bind _output_get_5 (set `self.Light Color` (struct :`R` 0.379167 :`G` 0.368174 :`B` 0.049371 :`A` 1.0)))
            (`LightComponent.SetLightColor` _spotlight _output_get_5 true)
            (`LightComponent.SetLightColor` (`self.PointLight`) _output_get_5 true)
            (`PrimitiveComponent.SetMaterial` (`self.Light`) (`self.Element Index`) "/Game/Materials/Colour_Mat/Material_Colour_Yellow.Material_Colour_Yellow")))))))