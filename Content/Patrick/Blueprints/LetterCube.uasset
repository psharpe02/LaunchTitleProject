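; LetterCube is a cube actor with configurable decals that makes the first-person character's arms show pushing when a hand touches it.
; On BeginPlay it applies a visibility flag and two materials to its decal components.
; Capsule begin and end overlap events check whether either of the character's hand collisions still overlaps the capsule, then set the Pushing flag on FPArms accordingly.
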(event `self.ReceiveBeginPlay`
  (bind _decal2 (`self.Decal2`))
  (`SceneComponent.SetVisibility` _decal2 (`self.DecalVisable?`) false)
  (`SceneComponent.SetVisibility` (`self.Decal2`) (`self.DecalVisable?`) false)
  (`SceneComponent.SetVisibility` (`self.Decal3`) (`self.DecalVisable?`) false)
  (`DecalComponent.SetDecalMaterial` _decal2 (`self.Decal Material`))
  (`DecalComponent.SetDecalMaterial` (`self.Decal3`) (`self.Decal2 Material`)))

(event `self.Capsule.OnComponentBeginOverlap`
  (params (OverlappedComponent :type "PrimitiveComponent Object Reference") (OtherActor :type "Actor Object Reference") (OtherComp :type "PrimitiveComponent Object Reference") (OtherBodyIndex :type Integer) (bFromSweep :type Boolean) (SweepResult :type "HitResult Structure (by ref)"))
  (bind _capsule (`self.Capsule`))
  (bind _asfirst_person_character (cast `/Game/FirstPersonBP/Blueprints/FirstPersonCharacter` OtherActor))
  (if (or (`PrimitiveComponent.IsOverlappingComponent` (`/Game/FirstPersonBP/Blueprints/FirstPersonCharacter.LHand Collision` _asfirst_person_character) _capsule) (`PrimitiveComponent.IsOverlappingComponent` (`/Game/FirstPersonBP/Blueprints/FirstPersonCharacter.RHand Collision` _asfirst_person_character) _capsule))
    (bind _fparms (`/Game/FirstPersonBP/Blueprints/FirstPersonCharacter.FPArms` _asfirst_person_character))
    (set `/Game/Animation/FirstPersonArms/FirstPersonArms.Pushing?` true _fparms)
    (else
      (set `/Game/Animation/FirstPersonArms/FirstPersonArms.Pushing?` false _fparms))))

(event `self.Capsule.OnComponentEndOverlap`
  (params (OverlappedComponent :type "PrimitiveComponent Object Reference") (OtherActor :type "Actor Object Reference") (OtherComp :type "PrimitiveComponent Object Reference") (OtherBodyIndex :type Integer))
  (bind _capsule (`self.Capsule`))
  (bind _asfirst_person_character (cast `/Game/FirstPersonBP/Blueprints/FirstPersonCharacter` OtherActor))
  (if (or (`PrimitiveComponent.IsOverlappingComponent` (`/Game/FirstPersonBP/Blueprints/FirstPersonCharacter.LHand Collision` _asfirst_person_character) _capsule) (`PrimitiveComponent.IsOverlappingComponent` (`/Game/FirstPersonBP/Blueprints/FirstPersonCharacter.RHand Collision` _asfirst_person_character) _capsule))
    (bind _fparms (`/Game/FirstPersonBP/Blueprints/FirstPersonCharacter.FPArms` _asfirst_person_character))
    (set `/Game/Animation/FirstPersonArms/FirstPersonArms.Pushing?` true _fparms)
    (else
      (set `/Game/Animation/FirstPersonArms/FirstPersonArms.Pushing?` false _fparms))))

(fn `UserConstructionScript`)